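; BP_NPC is an AI character with health, an ability system and a spline patrol route.
; BeginPlay seeds the blackboard BehaviorState, binds the health component's death event and links the health widget to the NPC.
; Death sets the Dead state, clears abilities, removes the capsule, fires a death GameplayCue and destroys the actor after a delay.
; IncrementPatrolIndex wraps through spline points, flipping PatrolDirection at each wrap to zero.
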(event Custom|OnNPCDeath_Event
  (AI|Components|Blackboard|SetValueasEnum (AI|GetBlackboard 0) (Utilities|Name|MakeLiteralName "BehaviorState") (Utilities|Enum|LiteralenumEBehaviorStateTypes "Dead"))
  (Class|AbilitySystemComponent|ClearAllAbilities (Ability|GetAbilitySystemComponent 0))
  (Components|DestroyComponent (Variables|Default|GetCapsuleComponent))
  (GameplayCue|ExecuteGameplayCueOnActor(Burst) self "(TagName=\"GameplayCue.NPC.Death\")" (Ability|GameplayCue|MakeGameplayCueParameters 0.0))
  (Utilities|FlowControl|Delay 5.0)
  (Actor|DestroyActor))

(event EventBeginPlay
  (AI|Components|Blackboard|SetValueasEnum (AI|GetBlackboard (AI|GetAIController self)) (Utilities|Name|MakeLiteralName "BehaviorState") (Variables|Default|GetStartBehaviorState))
  (EventDispatchers|AssignOnNPCDeath (Variables|Default|GetHealthComponent) (delegate Custom|OnNPCDeath_Event))
  (bind _aswbp_health (Utilities|Casting|CastToWBP_Health (UserInterface|GetUserWidgetObject (Variables|Default|GetHealthWidgetComponent))))
  (Variables|/Game/UI/Health/WBP_Health.WBP_Health_C|SetOwnerNPC _aswbp_health self))

(event Collision|EventActorBeginOverlap
  (params (OtherActor :type Actor%20Object%20Reference)))

(event EventTick
  (params (DeltaSeconds :type Float%20%28single-precision%29)))

(fn ConstructionScript)

(fn IncrementPatrolIndex
  (bind _output_get (Variables|PatrolMovement|SetPatrolIndex (Math|Float|Truncate (.Remainder (Math|Float|Division(WholeandRemainder) (Math|Conversions|ToFloat(Integer) (+ (Variables|PatrolMovement|GetPatrolIndex) 1)) (Math|Conversions|ToFloat(Integer) (Spline|GetNumberOfSplinePoints (Variables|/Script/Testovoe.PatrolPath|GetPatrolRout (Variables|Default|GetpatrolPath)))))))))
  (if (== _output_get 0)
    (Variables|PatrolMovement|SetPatrolDirection (not (Variables|PatrolMovement|GetPatrolDirection)))))