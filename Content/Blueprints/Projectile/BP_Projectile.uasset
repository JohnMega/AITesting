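; BP_Projectile is a team-aware projectile that damages NPCs of other teams.
; When its sphere overlaps an NPC, it compares that NPC's team ID with the owner NPC's, then applies a fixed amount of damage and destroys itself if they differ.
; Overlaps with teammates or non-NPC actors, or without a valid owner, are ignored, and the projectile otherwise self-destructs when its lifetime delay ends.
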(event OnComponentBeginOverlap(Sphere)
  (params (OverlappedComponent :type Primitive%20Component%20Object%20Reference) (OtherActor :type Actor%20Object%20Reference) (OtherComp :type Primitive%20Component%20Object%20Reference) (OtherBodyIndex :type Integer) (bFromSweep :type Boolean) (SweepResult :type Hit%20Result%20Structure%20%28by%20ref%29))
  (bind _ownernpc (Variables|Default|GetOwnerNPC))
  (bind _asnpc (Utilities|Casting|CastToNPC OtherActor))
  (Utilities|IsValid _ownernpc
    (:Is%20Valid
      (if (!= (.teamid (Variables|/Script/Testovoe.NPC|GetTeamID _asnpc)) (.teamid (Variables|/Script/Testovoe.NPC|GetTeamID _ownernpc)))
        (Game|Damage|ApplyDamage _asnpc 2e+01 0 0)
        (Actor|DestroyActor)))))

(event EventBeginPlay
  (Utilities|FlowControl|Delay (Variables|Default|GetLifetime))
  (Actor|DestroyActor))

(event Collision|EventActorBeginOverlap
  (params (OtherActor :type Actor%20Object%20Reference)))

(event EventTick
  (params (DeltaSeconds :type Float%20%28single-precision%29)))

(fn ConstructionScript)